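; BP_FieldSystem is a Chaos field system actor that breaks and scatters Geometry Collection fragments around its location on BeginPlay.
; It applies an external strain field with linear radial falloff to break clusters within SphereRadius.
; It then applies linear velocity from a radial vector multiplied by a matching falloff mask, pushing pieces outward.
; A long-lived debug sphere draws the affected radius.
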(event `self.ReceiveBeginPlay`
  (bind _returnvalue (`self.K2_GetActorLocation`))
  (bind _fieldsystemcomponent (`self.FieldSystemComponent`))
  (bind _fieldsystemmetadatafilter (`self.FieldSystemMetaDataFilter`))
  ; Break the cluster forces with External Strain
  (`FieldSystemComponent.ApplyPhysicsField` _fieldsystemcomponent true "Field_ExternalClusterStrain" _fieldsystemmetadatafilter (`RadialFalloff.SetRadialFalloff` (`self.RadialFalloff (External Strain)`) 5000.0 0.0 1.0 0.0 (`self.Sphere Radius`) _returnvalue "Field_Falloff_Linear"))
  ; Scatter the fragments with a Radial Vector
  (`FieldSystemComponent.ApplyPhysicsField` _fieldsystemcomponent true "Field_LinearVelocity" _fieldsystemmetadatafilter (`OperatorField.SetOperatorField` (`self.OperatorField`) 1.0 (`RadialVector.SetRadialVector` (`self.RadialVector`) 250.0 _returnvalue) (`RadialFalloff.SetRadialFalloff` (`self.RadialFalloff (Velocity Mask)`) 1.0 0.0 1.0 0.0 (`self.Sphere Radius`) _returnvalue "Field_Falloff_Linear") "Field_Multiply"))
  (`KismetSystemLibrary.DrawDebugSphere` (`self.K2_GetActorLocation`) (`self.Sphere Radius`) 12 (struct :`R` 1.0 :`G` 1.0 :`B` 1.0 :`A` 1.0) 300.0))

(fn `UserConstructionScript`)