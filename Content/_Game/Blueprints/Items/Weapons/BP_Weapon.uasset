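; BP_Weapon is a weapon Blueprint that creates physics fields at a given location to fracture destructible geometry.
; Its CreateWeaponFields event applies a linear-falloff radial external strain to break cluster bonds.
; It then scatters the fragments with a linear velocity field, multiplying a radial vector by a second radial falloff mask so the push fades with distance.
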(event `self.CreateWeaponFields`
  (params (FieldLocation :type "Vector Structure (by ref)"))
  (bind _fieldsystem (`self.FieldSystem`))
  (bind _fieldsystemmetadatafilter (`self.FieldSystemMetaDataFilter`))
  ; Break the cluster forces with External Strain
  (`FieldSystemComponent.ApplyPhysicsField` _fieldsystem true "Field_ExternalClusterStrain" _fieldsystemmetadatafilter (`RadialFalloff.SetRadialFalloff` (`self.RadialFalloff (External Strain)`) 1000000.0 0.0 1.0 0.0 (`self.SphereRadius`) FieldLocation "Field_Falloff_Linear"))
  ; Scatter the fragments with a Radial Vector
  (`FieldSystemComponent.ApplyPhysicsField` _fieldsystem true "Field_LinearVelocity" _fieldsystemmetadatafilter (`OperatorField.SetOperatorField` (`self.OperatorField (Multiply)`) 1.0 (`RadialVector.SetRadialVector` (`self.RadialVector`) 200.0 FieldLocation) (`RadialFalloff.SetRadialFalloff` (`self.RadialFalloff (Velocity Mask)`) 1.0 0.0 1.0 0.0 (`self.SphereRadius`) FieldLocation "Field_Falloff_Linear") "Field_Multiply")))

(fn `UserConstructionScript`)